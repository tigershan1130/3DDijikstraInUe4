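; Clickable sphere that can be picked as the start or end point stored in the MainUI widget.
; A click fills the empty start slot first, then the end slot, with the sphere's world location and swaps its material to match.
; Clicking an assigned sphere restores the basic material and frees its slot.
; An if chain checks inverted local flags (false means assigned) and the widget's (-1,-1,-1) empty sentinel.
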(event `self.Sphere.OnClicked`
  (params (TouchedComponent :type "PrimitiveComponent Object Reference") (ButtonPressed :type "Key Structure"))
  (bind _returnvalue (`SceneComponent.K2_GetComponentLocation` TouchedComponent))
  (bind _foundwidgets (`WidgetBlueprintLibrary.GetAllWidgetsOfClass` "/Game/UI/MainUI.MainUI_C"))
  (bind _output (`|GetArrayItem` _foundwidgets))
  (if (and (`KismetMathLibrary.EqualExactly_VectorVector` (`/Game/UI/MainUI.StartPoint` _output) (-1.0 -1.0 -1.0)) (`KismetMathLibrary.EqualExactly_VectorVector` (`/Game/UI/MainUI.EndPoint` _output) (-1.0 -1.0 -1.0)) (== (`self.StartPoint`) true) (== (`self.EndPoint`) true))
    (`PrimitiveComponent.SetMaterial` TouchedComponent 0 "/Game/Materials/StartPointMaterial.StartPointMaterial")
    (set `/Game/UI/MainUI.StartPoint` _returnvalue _output)
    (set `self.StartPoint` false)
    (elif (and (`KismetMathLibrary.NotEqualExactly_VectorVector` (`/Game/UI/MainUI.StartPoint` _output) (-1.0 -1.0 -1.0)) (`KismetMathLibrary.EqualExactly_VectorVector` (`/Game/UI/MainUI.EndPoint` _output) (-1.0 -1.0 -1.0)) (== (`self.StartPoint`) false) (== (`self.EndPoint`) true))
      (`PrimitiveComponent.SetMaterial` TouchedComponent 0 "/Engine/BasicShapes/BasicShapeMaterial.BasicShapeMaterial")
      (set `/Game/UI/MainUI.StartPoint` (-1.0 -1.0 -1.0) _output)
      (set `self.StartPoint` true)
      (elif (and (`KismetMathLibrary.NotEqualExactly_VectorVector` (`/Game/UI/MainUI.StartPoint` _output) (-1.0 -1.0 -1.0)) (`KismetMathLibrary.EqualExactly_VectorVector` (`/Game/UI/MainUI.EndPoint` _output) (-1.0 -1.0 -1.0)) (== (`self.StartPoint`) true) (== (`self.EndPoint`) true))
        (`PrimitiveComponent.SetMaterial` TouchedComponent 0 "/Game/Materials/EndPointMaterial.EndPointMaterial")
        (set `/Game/UI/MainUI.EndPoint` _returnvalue _output)
        (set `self.EndPoint` false)
        (elif (and (`KismetMathLibrary.NotEqualExactly_VectorVector` (`/Game/UI/MainUI.StartPoint` _output) (-1.0 -1.0 -1.0)) (`KismetMathLibrary.NotEqualExactly_VectorVector` (`/Game/UI/MainUI.EndPoint` _output) (-1.0 -1.0 -1.0)) (== (`self.StartPoint`) false) (== (`self.EndPoint`) true))
          (`PrimitiveComponent.SetMaterial` TouchedComponent 0 "/Engine/BasicShapes/BasicShapeMaterial.BasicShapeMaterial")
          (set `/Game/UI/MainUI.StartPoint` (-1.0 -1.0 -1.0) _output)
          (set `self.StartPoint` true)
          (elif (and (`KismetMathLibrary.NotEqualExactly_VectorVector` (`/Game/UI/MainUI.StartPoint` _output) (-1.0 -1.0 -1.0)) (`KismetMathLibrary.NotEqualExactly_VectorVector` (`/Game/UI/MainUI.EndPoint` _output) (-1.0 -1.0 -1.0)) (== (`self.StartPoint`) true) (== (`self.EndPoint`) false))
            (`PrimitiveComponent.SetMaterial` TouchedComponent 0 "/Engine/BasicShapes/BasicShapeMaterial.BasicShapeMaterial")
            (set `/Game/UI/MainUI.EndPoint` (-1.0 -1.0 -1.0) _output)
            (set `self.EndPoint` true)
            (elif (and (`KismetMathLibrary.EqualExactly_VectorVector` (`/Game/UI/MainUI.StartPoint` _output) (-1.0 -1.0 -1.0)) (`KismetMathLibrary.NotEqualExactly_VectorVector` (`/Game/UI/MainUI.EndPoint` _output) (-1.0 -1.0 -1.0)) (== (`self.StartPoint`) true) (== (`self.EndPoint`) true))
              (`PrimitiveComponent.SetMaterial` TouchedComponent 0 "/Game/Materials/StartPointMaterial.StartPointMaterial")
              (set `/Game/UI/MainUI.StartPoint` _returnvalue _output)
              (set `self.StartPoint` false)
              (elif (and (`KismetMathLibrary.EqualExactly_VectorVector` (`/Game/UI/MainUI.StartPoint` _output) (-1.0 -1.0 -1.0)) (`KismetMathLibrary.NotEqualExactly_VectorVector` (`/Game/UI/MainUI.EndPoint` _output) (-1.0 -1.0 -1.0)) (== (`self.StartPoint`) true) (== (`self.EndPoint`) false))
                (`PrimitiveComponent.SetMaterial` TouchedComponent 0 "/Engine/BasicShapes/BasicShapeMaterial.BasicShapeMaterial")
                (set `/Game/UI/MainUI.EndPoint` (-1.0 -1.0 -1.0) _output)
                (set `self.EndPoint` true)))))))))

(fn `UserConstructionScript`)